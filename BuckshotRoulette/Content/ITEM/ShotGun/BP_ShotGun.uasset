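; BP_ShotGun is a clickable shotgun actor that rises and opens a UI widget when clicked.
; BeginPlay enables mouse click events on the player controller.
; Each click on the Shotgun component lifts the actor along Z without supplying a rotation, then adds a new WBP_MainWidget to the viewport.
; The ShotLocRot event is empty, and leftover nodes for moving, rotating and lerping Shot are disconnected.
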(event OnClicked(Shotgun)
  (params (TouchedComponent :type Primitive%20Component%20Object%20Reference) (ButtonPressed :type Key%20Structure :default "None"))
  (bind _returnvalue (Transformation|GetActorLocation))
  (bind _output_get (Variables|Default|SetNewloc (Math|Vector|MakeVector (.x _returnvalue) (.y _returnvalue) (+ (.z _returnvalue) 8e+01))))
  (Transformation|SetActorLocationAndRotation _output_get "0, 0, 0")
  (bind _returnvalue_2 (UserInterface|CreateWidget "/Game/Assets/UI/WBP_MainWidget.WBP_MainWidget_C"))
  (UserInterface|Viewport|AddtoViewport _returnvalue_2 0))

(event Custom|ShotLocRot)

(event Collision|EventActorBeginOverlap
  (params (OtherActor :type Actor%20Object%20Reference)))

(event EventTick
  (params (DeltaSeconds :type Float%20%28single-precision%29)))

(event EventBeginPlay
  (Variables|/Script/Engine.PlayerController|SetbEnableClickEvents (Game|GetPlayerController 0) true))

(fn ConstructionScript)